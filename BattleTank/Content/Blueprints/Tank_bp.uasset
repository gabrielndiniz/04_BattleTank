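; Tank pawn Blueprint that assembles the player-controllable tank and routes its input.
; BeginPlay assigns turret, barrel and track meshes, gives both tracks a physical material override, then hands the component references to setter functions.
; Aim axes rotate an azimuth gimbal and spring arm for the camera.
; Throttle axes drive each track separately, fly-by-wire forward input goes to TankMovementComponent, and the Fire action calls Fire.
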(event EventBeginPlay
  (Utilities|FlowControl|Sequence
    (:then_0
      (Components|StaticMesh|SetStaticMesh (Variables|Default|GetTurret) "/Game/vehicles_3d/TankStandard/tank_fbx_Turret.tank_fbx_Turret"))
    (:then_1
      (Utilities|FlowControl|Sequence
        (:then_0
          (Components|StaticMesh|SetStaticMesh (Variables|Default|GetBarrel) "/Game/vehicles_3d/TankStandard/tank_fbx_Barrel.tank_fbx_Barrel"))
        (:then_1
          (Utilities|FlowControl|Sequence
            (:then_0
              (Components|StaticMesh|SetStaticMesh (Variables|Default|GetLeft%20Track) "/Game/vehicles_3d/TankStandard/tank_fbx_Track.tank_fbx_Track"))
            (:then_1
              (Utilities|FlowControl|Sequence
                (:then_0
                  (Components|StaticMesh|SetStaticMesh (Variables|Default|GetRight%20Track) "/Game/vehicles_3d/TankStandard/tank_fbx_Track.tank_fbx_Track"))
                (:then_1
                  (Utilities|FlowControl|Sequence
                    (:then_0
                      (Class|PrimitiveComponent|SetPhysMaterialOverride (Variables|Default|GetLeft%20Track) "/Game/Materials/Track.Track"))
                    (:then_1
                      (Utilities|FlowControl|Sequence
                        (:then_0
                          (Class|PrimitiveComponent|SetPhysMaterialOverride (Variables|Default|GetRight%20Track) "/Game/Materials/Track.Track"))
                        (:then_1
                          (Class|Tank|SetTurretReference (Variables|Default|GetTurret))
                          (Class|Tank|SetBarrelReference (Variables|Default|GetBarrel))
                          (Class|Tank|SetTrackReference (Variables|Default|GetLeft%20Track))
                          (Class|Tank|SetTrackReference (Variables|Default|GetRight%20Track)))))))))))))))

(event Input|ActionEvents|InputActionFire
  (params (Key :type Key%20Structure :default "None"))
  ;[1 1 1] Aiming Input Binding
  (:Pressed
    (Class|Tank|Fire)))

(event Input|AxisEvents|InputAxisAimAzimuth
  (params (AxisValue :type Float%20%28single-precision%29))
  ;[1 1 1] Aiming Input Binding
  (Transformation|AddLocalRotation (Variables|Default|GetAzimuth%20Gimbal) (Math|Rotator|MakeRotator 0.0 0.0 AxisValue) false false))

(event Input|AxisEvents|InputAxisAimElevation
  (params (AxisValue :type Float%20%28single-precision%29))
  ;[1 1 1] Aiming Input Binding
  (Transformation|AddLocalRotation (Variables|Default|GetSpringArm) (Math|Rotator|MakeRotator 0.0 AxisValue 0.0) false false))

(event Input|AxisEvents|InputAxisLeftTrackThrottle
  (params (AxisValue :type Float%20%28single-precision%29))
  ;[1 1 1] Movement Component
  (Class|TankTrack|SetThrottle (Variables|Default|GetLeft%20Track) AxisValue))

(event Input|AxisEvents|InputAxisRightTrackThrottle
  (params (AxisValue :type Float%20%28single-precision%29))
  ;[1 1 1] Movement Component
  (Class|TankTrack|SetThrottle (Variables|Default|GetRight%20Track) AxisValue))

(event Input|AxisEvents|InputAxisFly-By-WireMoveForward
  (params (AxisValue :type Float%20%28single-precision%29))
  ;[1 1 1] Movement Component
  (Class|TankMovementComponent|IntendMoveForward (Variables|Default|GetTankMovementComponent) AxisValue))

(fn ConstructionScript)